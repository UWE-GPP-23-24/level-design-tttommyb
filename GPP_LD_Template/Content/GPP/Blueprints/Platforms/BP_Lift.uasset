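; BP_Lift is a platform actor that carries its Platform component from StartPoint toward EndPoint.
; BeginPlay snaps the platform to the start, sets the current and target points, and sets the timeline play rate from MoveSpeed.
; MoveUp plays the timeline from the start, lerping world location without sweep, while Reset teleports back and stops it.
; Nothing here calls MoveUp or reverses direction.
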(event `self.ReceiveBeginPlay`
  ;[0.4491 0.8591 1] Init
  ;;[0.4491 0.8591 1] Initialise to the start location
  (`TypedElementListLibrary.Reset` (struct))
  ;;[0.4491 0.8591 1] Set target and current points
  (set `self.TargetPoint` (`self.EndPoint`))
  (set `self.IsHeadingToEndPoint` true)
  (set `self.CurrentPoint` (`self.StartPoint`))
  (`TimelineComponent.SetPlayRate` (`self.Timeline`) (`self.MoveSpeed`)))

(event `MoveUp`
  ;[0.4491 0.8591 1] Move to target points
  (bind (_direction _alpha) (`Timeline|Timeline` :!via `PlayFromStart`)
    (:`Update`
      ;;[0.4491 0.8591 1] Lerp between points
      (`SceneComponent.K2_SetWorldLocation` (`self.Platform`) (`KismetMathLibrary.VLerp` (`SceneComponent.K2_GetComponentLocation` (`self.CurrentPoint`)) (`SceneComponent.K2_GetComponentLocation` (`self.TargetPoint`)) _alpha) false false))))

(event `Reset`
  (`SceneComponent.K2_SetWorldLocation` (`self.Platform`) (`SceneComponent.K2_GetComponentLocation` (`self.StartPoint`)) false true)
  (`TimelineComponent.Stop` (`self.Timeline`)))

(fn `UserConstructionScript`
  (`parent.UserConstructionScript`))