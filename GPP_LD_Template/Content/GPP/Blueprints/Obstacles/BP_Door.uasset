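; BP_Door is an obstacle that opens once every linked key is collected.
; Tick polls the Keys array until Opened is set, then runs a short delayed sequence that freezes player movement, blends the view to Camera and calls OpenDoor.
; OpenDoor plays a timeline that lerps Platform from StartPoint to EndPoint, and the sequence then returns view and walking to the player.
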(event `self.ReceiveBeginPlay`
  (`SceneComponent.K2_SetWorldLocation` (`self.Platform`) (`SceneComponent.K2_GetComponentLocation` (`self.StartPoint`)) false true))

(event `Open Door`
  (bind (_direction _alpha) (`Timeline|Timeline`)
    (:`Update`
      (`SceneComponent.K2_SetWorldLocation` (`self.Platform`) (`KismetMathLibrary.VLerp` (`SceneComponent.K2_GetComponentLocation` (`self.StartPoint`)) (`SceneComponent.K2_GetComponentLocation` (`self.EndPoint`)) _alpha) false false))))

(event `self.ReceiveTick`
  (params (DeltaSeconds :type "Float (single-precision)"))
  (bind _returnvalue (`GameplayStatics.GetPlayerCharacter` 0))
  (bind _returnvalue_2 (`GameplayStatics.GetPlayerController` 0))
  (bind _charactermovement (`Character.CharacterMovement` _returnvalue))
  (if (not (`self.Opened`))
    (set `self.Collected All` true)
    (for _array_element (`self.Keys`)
      (if (== (`/Game/GPP/Blueprints/Collectibles/BP_Key.Collected` _array_element) false)
        (set `self.Collected All` false)))
    (if (`self.Collected All`)
      (`CharacterMovementComponent.SetMovementMode` _charactermovement "MOVE_None" 0)
      (`PlayerController.SetViewTargetWithBlend` _returnvalue_2 (`self.Camera`) 0.0 "VTBlend_EaseIn" 0.5 false)
      (`KismetSystemLibrary.Delay` 1.0)
      (`self.Open Door`)
      (`KismetSystemLibrary.Delay` 1.0)
      (`PlayerController.SetViewTargetWithBlend` _returnvalue_2 _returnvalue 1.0 "VTBlend_Cubic" 0.5 false)
      (`CharacterMovementComponent.SetMovementMode` _charactermovement "MOVE_Walking" 0)
      (set `self.Opened` true))))

(fn `UserConstructionScript`)