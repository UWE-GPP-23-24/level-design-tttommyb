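; Exploding platform obstacle that detonates when its fuse runs out and later respawns.
; While triggered, Tick counts the fuse down, pausing whenever the freezable component reports it frozen.
; At zero it calls the explodable component, clears the trigger, then after a delay spawns a fresh copy of itself at its transform.
; The trigger flag is never set in this graph.
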(event `self.ReceiveTick`
  (params (DeltaSeconds :type "Float (single-precision)"))
  ;[0.4491 0.8591 1] Tick
  ;;[0.4491 0.8591 1] Check if timer can tick down
  (if (and (`self.IsTriggered`) (not (`/Game/GPP/Blueprints/Components/BP_FreezableComponent.GetIsFrozen` (`self.BP_FreezableComponent`))))
    ;;[0.4491 0.8591 1] Count down fuse timer
    (bind _output_get (set `self.FuseTimer` (- (`self.FuseTimer`) DeltaSeconds)))
    (if (< _output_get 0.0)
      ;;[0.4491 0.8591 1] Explode
      (`/Game/GPP/Blueprints/Components/BP_ExplodableComponent.Explode` (`self.BP_ExplodableComponent`))
      (set `self.IsTriggered` false)
      (set `self.FuseTimer` 0.0)
      (`KismetSystemLibrary.Delay` 10.0)
      (`|SpawnActorFromClass` "BP_Exploding_Platform_C" (`self.GetTransform`) "Undefined" "MultiplyWithRoot" null null))))

(fn `UserConstructionScript`
  (`parent.UserConstructionScript`))